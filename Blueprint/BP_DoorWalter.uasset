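; BP_DoorWalter is a hinged door that opens and closes on interaction, gated by blue and red key requirements.
; Interaction checks the key counts in GM_ModeJuego against the door's own requirements, then toggles IsOpen and the target yaw without consuming keys.
; Tick continuously eases the Scene component's yaw toward that target with FInterpTo at SpeedDoor, swinging the door a quarter turn.
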(event `/Game/Interface/Interaction.Interaction`
  (bind _asgm_mode_juego (cast `/Game/GameMode/GM_ModeJuego` (`GameplayStatics.GetGameMode`) :!pure true))
  (if (>= (`/Game/GameMode/GM_ModeJuego.LlavesAzules` _asgm_mode_juego) (`self.LlavesAzules`))
    (if (>= (`/Game/GameMode/GM_ModeJuego.LlavesRojas` _asgm_mode_juego) (`self.LlavesRojas`))
      (if (`self.IsOpen`)
        (set `self.TargetAngle` 0.0)
        (set `self.IsOpen` false)
        (else
          (set `self.TargetAngle` -90.0)
          (set `self.IsOpen` true))))))

(event `self.ReceiveTick`
  (params (DeltaSeconds :type "Float (single-precision)"))
  (bind _scene (`self.Scene`))
  (bind (_relativerotation_roll _relativerotation_pitch _relativerotation_yaw) (`KismetMathLibrary.BreakRotator` (`SceneComponent.RelativeRotation` _scene)))
  (`SceneComponent.K2_SetRelativeRotation` _scene (`KismetMathLibrary.MakeRotator` 0.0 0.0 (`KismetMathLibrary.FInterpTo` _relativerotation_yaw (`self.TargetAngle`) DeltaSeconds (`self.SpeedDoor`))) false false))

(fn `UserConstructionScript`)