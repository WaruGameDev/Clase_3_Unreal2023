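; BP_Jugador is the player character, handling movement, camera look, jumping, door interaction and coin pickup.
; Custom events apply movement relative to control rotation, controller look input and jumping; no input bindings live here.
; Abrir sends AbrirPuertaMessage to overlapping actors that implement the Interaction interface.
; Overlapping a BP_Moneda adds one coin through the GM_ModeJuego reference cached on BeginPlay.
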(event `MovimientoAdelanteYAtras`
  (params (ScaleValue :type "Float (single-precision)"))
  (bind (_returnvalue_roll _returnvalue_pitch _returnvalue_yaw) (`KismetMathLibrary.BreakRotator` (`self.GetControlRotation`)))
  (`self.AddMovementInput` (`KismetMathLibrary.GetForwardVector` (`KismetMathLibrary.MakeRotator` 0.0 0.0 _returnvalue_yaw)) ScaleValue))

(event `Abrir`
  ;[1 1 1] Evento custom para definir el BP Interface y que evento se ejecutara al final
  (for _array_element (`self.GetOverlappingActors` null)
    (if (`KismetSystemLibrary.DoesImplementInterface` _array_element "/Game/Interface/Interaction.Interaction_C")
      (message `/Game/Interface/Interaction.AbrirPuerta` _array_element))))

(event `MovimientoDerechaIzquierda`
  (params (ScaleValue :type "Float (single-precision)"))
  (bind (_returnvalue_roll _returnvalue_pitch _returnvalue_yaw) (`KismetMathLibrary.BreakRotator` (`self.GetControlRotation`)))
  (`self.AddMovementInput` (`KismetMathLibrary.GetRightVector` (`KismetMathLibrary.MakeRotator` _returnvalue_roll 0.0 _returnvalue_yaw)) ScaleValue))

(event `MouseLook`
  (params (X :type "Float (single-precision)") (Y :type "Float (single-precision)"))
  (`self.AddControllerYawInput` X)
  (`self.AddControllerPitchInput` Y))

(event `JumpPlayer`
  (params (Condition :type Boolean))
  (if Condition
    (`self.Jump`)
    (else
      (`self.StopJumping`))))

(event `self.ReceiveActorBeginOverlap`
  (params (OtherActor :type "Actor Object Reference"))
  (cast `/Game/Blueprint/BP_Moneda` OtherActor)
  (`/Game/GameMode/GM_ModeJuego.AgregarMoneda` (`self.As GM Mode Juego`) 1))

(event `self.ReceiveBeginPlay`
  (set `self.As GM Mode Juego` (cast `/Game/GameMode/GM_ModeJuego` (`GameplayStatics.GetGameMode`) :!pure true)))

(fn `UserConstructionScript`)