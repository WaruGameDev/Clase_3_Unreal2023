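; GM_ModeJuego is a game mode that holds the player's health, coin count and red and blue key counts.
; On BeginPlay it creates the UIVida widget, stores a reference and adds it to the viewport.
; AñadirVida and QuitarVida events change health by a fixed step, clamped between zero and Max.
; Functions increment each key counter or add a given amount of coins, printing the new coin total.
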(event `self.ReceiveBeginPlay`
  (bind _returnvalue (`|CreateWidget` "/Game/UMG/UIVida.UIVida_C" (`self.Owning Player`)))
  (bind _output_get (set `self.UIWidgetReference` _returnvalue))
  (`UserWidget.AddToViewport` _output_get 0))

(event `/Game/Interface/BPI_SistemaSalud.AñadirVida`
  (set `self.Vida` (`KismetMathLibrary.FClamp` (+ (`self.Vida`) 10.0) 0.0 (`self.Max`))))

(event `/Game/Interface/BPI_SistemaSalud.QuitarVida`
  (set `self.Vida` (`KismetMathLibrary.FClamp` (- (`self.Vida`) 10.0) 0.0 (`self.Max`))))

(fn `AgregarLlaveAzul`
  (`/Engine/EditorBlueprintResources/StandardMacros.IncrementInt` (`self.LlavesAzules`)))

(fn `AgregarLlaveRoja`
  (`/Engine/EditorBlueprintResources/StandardMacros.IncrementInt` (`self.LlavesRojas`)))

(fn `AgregarMoneda`
  (params (Cantidad :type Integer))
  (bind _output_get (set `self.ContMonedas` (+ Cantidad (`self.ContMonedas`))))
  (`KismetSystemLibrary.PrintString` (`KismetStringLibrary.Conv_IntToString` _output_get)))

(fn `UserConstructionScript`)