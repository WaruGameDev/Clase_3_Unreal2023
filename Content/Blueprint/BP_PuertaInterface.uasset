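; BP_PuertaInterface is a key-locked door that toggles between open and closed.
; ObtenerLlave grants the key; AbrirPuerta prints whether the key is held and, if so, flips the open state and target angle.
; Tick runs FInterpTo from the Scene component's relative yaw toward that angle at VelocidadPuerta, feeding the result into AddRelativeRotation as a yaw delta rather than setting it as absolute rotation.
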(event `/Game/Interface/BPI_Interaccion.AbrirPuerta`
  (if (`self.GetKey`)
    (`KismetSystemLibrary.PrintString` "Tienes la llave")
    (if (`self.IsOpened`)
      (set `self.Angulo` 0.0)
      (set `self.IsOpened` false)
      (else
        (set `self.Angulo` -90.0)
        (set `self.IsOpened` true)))
    (else
      (`KismetSystemLibrary.PrintString` "No tienes la llave"))))

(event `/Game/Interface/BPI_Interaccion.ObtenerLlave`
  (set `self.GetKey` true))

(event `self.ReceiveTick`
  (params (DeltaSeconds :type "Float (single-precision)"))
  (bind _scene (`self.Scene`))
  (bind (_relativerotation_roll _relativerotation_pitch _relativerotation_yaw) (`KismetMathLibrary.BreakRotator` (`SceneComponent.RelativeRotation` _scene)))
  (`SceneComponent.K2_AddRelativeRotation` _scene (`KismetMathLibrary.MakeRotator` 0.0 0.0 (`KismetMathLibrary.FInterpTo` _relativerotation_yaw (`self.Angulo`) DeltaSeconds (`self.VelocidadPuerta`))) false false))

(fn `UserConstructionScript`)