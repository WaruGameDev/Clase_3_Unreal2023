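; BP_DoorInterface is a key-locked door that swings open and closed through Blueprint Interface events.
; RecogerLlave sets the key flag on the door itself, and AbrirPuerta toggles the target yaw between closed and a quarter turn only when that flag is set.
; Tick eases the Scene component's relative yaw toward the target with FInterpTo at SpeedDoor, and debug prints report whether the key is held.
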(event `/Game/Interface/Interaction.AbrirPuerta`
  ;[1 1 1] Evento de BP Interface para abrir la puerta
  (if (`self.GetKey?`)
    (`KismetSystemLibrary.PrintString` "Puedes abrir la puerta :D")
    (if (`self.IsOpen`)
      (set `self.TargetAngle` 0.0)
      (set `self.IsOpen` false)
      (else
        (set `self.TargetAngle` -90.0)
        (set `self.IsOpen` true)))
    (else
      (`KismetSystemLibrary.PrintString` "No tienes la llave"))))

(event `self.ReceiveTick`
  (params (DeltaSeconds :type "Float (single-precision)"))
  (bind _scene (`self.Scene`))
  (bind (_relativerotation_roll _relativerotation_pitch _relativerotation_yaw) (`KismetMathLibrary.BreakRotator` (`SceneComponent.RelativeRotation` _scene)))
  ;[1 1 1] Animación de abrir puerta
  (`SceneComponent.K2_SetRelativeRotation` _scene (`KismetMathLibrary.MakeRotator` 0.0 0.0 (`KismetMathLibrary.FInterpTo` _relativerotation_yaw (`self.TargetAngle`) DeltaSeconds (`self.SpeedDoor`))) false false))

(event `/Game/Interface/Interaction.RecogerLlave`
  ;[1 1 1] Evento de BP Interface para recoger llave
  (set `self.GetKey?` true))

(fn `UserConstructionScript`)