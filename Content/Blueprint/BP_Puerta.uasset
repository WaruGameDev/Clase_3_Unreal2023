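; BP_Puerta is a door actor that only lets the player through once they have collected enough coins.
; On BeginPlay it caches the GM_ModeJuego game mode.
; When its Box component overlaps a BP_Jugador, it checks the game mode's coin counter against a threshold of three, then either destroys itself or prints a not-enough-coins message.
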(event `self.Box.OnComponentBeginOverlap`
  (params (OverlappedComponent :type "PrimitiveComponent Object Reference") (OtherActor :type "Actor Object Reference") (OtherComp :type "PrimitiveComponent Object Reference") (OtherBodyIndex :type Integer) (bFromSweep :type Boolean) (SweepResult :type "HitResult Structure (by ref)"))
  (cast `/Game/Blueprint/BP_Jugador` OtherActor)
  (if (>= (`/Game/GameMode/GM_ModeJuego.ContMonedas` (`self.As GM Mode Juego`)) 3)
    (`self.K2_DestroyActor`)
    (else
      (`KismetSystemLibrary.PrintString` "No tienes monedas suficientes"))))

(event `self.ReceiveBeginPlay`
  (set `self.As GM Mode Juego` (cast `/Game/GameMode/GM_ModeJuego` (`GameplayStatics.GetGameMode`) :!pure true)))

(fn `UserConstructionScript`)