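; BP_PlayerControllerClase is a player controller that routes Enhanced Input to the possessed BP_Jugador pawn.
; On BeginPlay it caches the pawn cast to BP_Jugador and, only if that succeeds, adds the IMC_InputClase mapping context.
; Move, jump and look actions call the pawn's own movement, jump and mouse-look functions, with the look Y axis inverted.
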(event `self.ReceiveBeginPlay`
  (bind _returnvalue (pcsubsystem `EnhancedInputLocalPlayerSubsystem` (`GameplayStatics.GetPlayerController` 0)))
  (bind _asbp_jugador (cast `/Game/Blueprint/BP_Jugador` (`self.K2_GetPawn`)))
  (set `self.As BP Jugador` _asbp_jugador)
  (`/Engine/EditorBlueprintResources/StandardMacros.IsValid` _returnvalue
    (:`Is Valid`
      (`EnhancedInputSubsystemInterface.AddMappingContext` _returnvalue "/Game/Input/IMC_InputClase.IMC_InputClase" 0 (struct)))))

(event `EnhancedInput|/Game/Input/Actions/IA_Move`
  (params (ActionValue :type "Vector2D Structure") (ElapsedSeconds :type "Float (double-precision)") (TriggeredSeconds :type "Float (double-precision)") (InputAction :type "InputAction Object Reference" :default "/Game/Input/Actions/IA_Move.IA_Move"))
  (bind _as_bp_jugador (`self.As BP Jugador`))
  (:`Triggered`
    (`/Game/Blueprint/BP_Jugador.MovimientoDerechaIzquierda` _as_bp_jugador ActionValue_X)
    (`/Game/Blueprint/BP_Jugador.MovimientoAdelanteYAtras` _as_bp_jugador ActionValue_Y)))

(event `EnhancedInput|/Game/Input/Actions/IA_Jump`
  (params (ActionValue :type Boolean) (ElapsedSeconds :type "Float (double-precision)") (TriggeredSeconds :type "Float (double-precision)") (InputAction :type "InputAction Object Reference" :default "/Game/Input/Actions/IA_Jump.IA_Jump"))
  (:`Triggered`
    (`/Game/Blueprint/BP_Jugador.JumpPlayer` (`self.As BP Jugador`) ActionValue)))

(event `EnhancedInput|/Game/Input/Actions/IA_Look`
  (params (ActionValue :type "Vector2D Structure") (ElapsedSeconds :type "Float (double-precision)") (TriggeredSeconds :type "Float (double-precision)") (InputAction :type "InputAction Object Reference" :default "/Game/Input/Actions/IA_Look.IA_Look"))
  (:`Triggered`
    (`/Game/Blueprint/BP_Jugador.MouseLook` (`self.As BP Jugador`) ActionValue_X (* ActionValue_Y -1.0))))

(fn `UserConstructionScript`)