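; Game mode Blueprint that holds shared player stats: health (Vida), a coin counter and counts of red and blue keys.
; The Daño and Salud events lower and raise health by a fixed step and print the result, with no clamping.
; AgregarMoneda adds a given amount of coins and prints the total, while the key functions increment their counters.
; Interaction is a stub returning zero, and BeginPlay only prints a debug greeting.
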(event `self.ReceiveBeginPlay`
  (set `self.Vida` (`self.Vida`))
  (`KismetSystemLibrary.PrintString` "Hello"))

(event `/Game/Interface/BPI_SistemaDeVida.Daño`
  (bind _output_get (set `self.Vida` (- (`self.Vida`) 10.0)))
  (`KismetSystemLibrary.PrintString` (`KismetStringLibrary.Conv_DoubleToString` _output_get)))

(event `/Game/Interface/BPI_SistemaDeVida.Salud`
  (bind _output_get (set `self.Vida` (+ (`self.Vida`) 10.0)))
  (`KismetSystemLibrary.PrintString` (`KismetStringLibrary.Conv_DoubleToString` _output_get)))

(fn `AgregarLlaveAzul`
  (`/Engine/EditorBlueprintResources/StandardMacros.IncrementInt` (`self.LlavesAzules`)))

(fn `AgregarLlaveRoja`
  (`/Engine/EditorBlueprintResources/StandardMacros.IncrementInt` (`self.LlavesRojas`)))

(fn `AgregarMoneda`
  (params (Cantidad :type Integer))
  (bind _output_get (set `self.ContMonedas` (+ Cantidad (`self.ContMonedas`))))
  (`KismetSystemLibrary.PrintString` (`KismetStringLibrary.Conv_IntToString` _output_get)))

(fn `Interaction`
  (params (Salud :type "Float (double-precision)" :default 0.0))
  (returns (NuevaSalud :type "Float (double-precision)"))
  (return 0.0))

(fn `UserConstructionScript`)